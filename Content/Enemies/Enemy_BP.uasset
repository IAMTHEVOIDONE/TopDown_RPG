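; Enemy Blueprint whose Type selects mesh and animation class in the construction script, with a skeleton warrior setup.
; Attack is gated by a DoOnce and plays a combo montage, using notifies to count down a random hit count, then stop it and reset the gate.
; GetDamage subtracts Health and plays a hit montage, or at zero ragdolls the mesh and destroys the actor after a delay.
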(event Custom|Attack
  (Utilities|FlowControl|DoOnce false :!label _label
    (:Completed
      (Variables|Default|SetAttackCount (Math|Random|RandomIntegerinRange 1 3))
      (Animation|Montage|PlayMontage (Variables|Character|GetMesh) "/Game/Enemies/SkeletonWarrior/Animations/Skeleton_ComboAttack_Montage.Skeleton_ComboAttack_Montage"
        (:OnNotifyBegin
          (bind _result (Math|Integer|DecrementInt (Variables|Default|GetAttackCount))
            (:%20%20
              (if (<= _result 0)
                (Animation|Montage|MontageStop (Components|SkeletalMesh|GetAnimInstance (Variables|Character|GetMesh)) 0.5 "/Game/Enemies/SkeletonWarrior/Animations/Skeleton_ComboAttack_Montage.Skeleton_ComboAttack_Montage")
                (goto _label Reset)))))))))

(event Custom|GetDamage
  (params (Damage :type Float%20%28double-precision%29))
  (bind _mesh (Variables|Character|GetMesh))
  (Development|PrintString "Hello")
  (bind _output_get (Variables|Default|SetHealth (- (Variables|Default|GetHealth) Damage)))
  (if (<= _output_get 0.0)
    (Physics|SetSimulatePhysics _mesh true)
    (Collision|SetCollisionProfileName (Variables|Character|GetMesh) "EnemyRagdoll" true :!class /Script/Engine.PrimitiveComponent)
    (Utilities|FlowControl|Delay 3.0)
    (Actor|DestroyActor)
    (else
      (Animation|Montage|PlayMontage _mesh "/Game/Enemies/SkeletonWarrior/Animations/Skeleton_Hit_Montage.Skeleton_Hit_Montage"))))

(event EventBeginPlay)

(event Collision|EventActorBeginOverlap
  (params (OtherActor :type Actor%20Object%20Reference)))

(event EventTick
  (params (DeltaSeconds :type Float%20%28single-precision%29)))

(fn ConstructionScript
  (bind _mesh (Variables|Character|GetMesh))
  (switch Utilities|FlowControl|Switch|SwitchonEnemyTypes (Variables|Default|GetType)
    (:NewEnumerator0
      (Components|SkeletalMesh|SetSkeletalMeshAsset _mesh "/Game/Enemies/SkeletonWarrior/Mesh/SkeletonWarrior.SkeletonWarrior")
      (Class|SkeletalMeshComponent|SetAnimClass _mesh "/Game/Enemies/SkeletonWarrior/BP/Skeleton_AnimBP.Skeleton_AnimBP_C"))))