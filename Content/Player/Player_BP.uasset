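; Player character Blueprint that handles Enhanced Input movement and a montage-based combo attack.
; BeginPlay adds the player mapping context through PlayerController_BP, and movement input drives the actor's forward and right vectors.
; Attack plays the combo montage, or buffers one follow-up if it is already playing.
; Each montage notify consumes that buffer, blending the montage out when no follow-up was pressed.
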(event EventBeginPlay)

(event Collision|EventActorBeginOverlap
  (params (OtherActor :type Actor%20Object%20Reference)))

(event EventTick
  (params (DeltaSeconds :type Float%20%28single-precision%29)))

(event Input|EnhancedActionEvents|EnhancedInputActionMovement_IA
  (params (ActionValue :type Vector%202D%20Structure) (ElapsedSeconds :type Float%20%28double-precision%29) (TriggeredSeconds :type Float%20%28double-precision%29) (InputAction :type Input%20Action%20Object%20Reference :default "/Game/Controls/Movement_IA.Movement_IA"))
  (:Triggered
    (Pawn|Input|AddMovementInput (Transformation|GetActorForwardVector) (.x ActionValue) false)
    (Pawn|Input|AddMovementInput (Transformation|GetActorRightVector) (.y ActionValue) false)))

(event Input|EnhancedActionEvents|EnhancedInputActionAttack
  (params (ActionValue :type Boolean) (ElapsedSeconds :type Float%20%28double-precision%29) (TriggeredSeconds :type Float%20%28double-precision%29) (InputAction :type Input%20Action%20Object%20Reference :default "/Game/Controls/Attack.Attack"))
  (:Started
    (if (Animation|Montage|MontageIsPlaying (Components|SkeletalMesh|GetAnimInstance (Variables|Character|GetMesh)) "/Game/Player/Animations/Player_ComboAttack_Montage.Player_ComboAttack_Montage")
      (Variables|Default|SetAttackIndex 1)
      (else
        (Animation|Montage|PlayMontage (Variables|Character|GetMesh) "/Game/Player/Animations/Player_ComboAttack_Montage.Player_ComboAttack_Montage"
          (:OnNotifyBegin
            (bind _result (Math|Integer|DecrementInt (Variables|Default|GetAttackIndex))
              (:%20%20
                (if (< _result 0)
                  (Animation|Montage|MontageStop (Components|SkeletalMesh|GetAnimInstance (Variables|Character|GetMesh)) 0.5 "/Game/Player/Animations/Player_ComboAttack_Montage.Player_ComboAttack_Montage")
                  (Variables|Default|SetAttackIndex 0))))))))))

(event EventBeginPlay
  (bind _asplayer_controller_bp (Utilities|Casting|CastToPlayerController_BP (Pawn|GetController)))
  (Input|AddMappingContext (PlayerController|LocalPlayerSubsystems|GetEnhancedInputLocalPlayerSubsystem _asplayer_controller_bp) "/Game/Controls/Player_IMC.Player_IMC" 0 "(bIgnoreAllPressedKeysUntilRelease=True,bForceImmediately=False)"))

(fn ConstructionScript)